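; Goomba-style enemy Blueprint for a Mario game that walks along X at reduced speed in a random starting direction.
; Non-player hits with an X normal reverse it, debounced by a DoOnce and short delay, and mirror the sprite by scale.
; On death it extends the parent logic: stops movement, pops upward with physics, ignores all collision, and increments BP_Mario's kill count.
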(event OnComponentHit(CapsuleComponent)
  (params (HitComponent :type Primitive%20Component%20Object%20Reference) (OtherActor :type Actor%20Object%20Reference) (OtherComp :type Primitive%20Component%20Object%20Reference) (NormalImpulse :type Vector :default "0, 0, 0") (Hit :type Hit%20Result%20Structure%20%28by%20ref%29))
  ;[1 1 1] Não mudar a direção se o encostar no player
  (if (!= OtherActor (Game|Player|GetPlayerPawn 0))
    (if (!= (.X (Math|Vector|BreakVector (.normal Hit))) 0.0)
      (Utilities|FlowControl|DoOnce false
        (:Completed
          (Variables|Default|SetMove_right (not (Variables|Default|GetMove_right)))
          (CallFunction|FacingDirection)
          (Utilities|FlowControl|Delay 0.1)
          (CallFunction|ResetDirectionChangeCheck))))))

(event Custom|ResetDirectionChangeCheck
  (Utilities|FlowControl|DoOnce false) ; enters at Reset
)

(event EventBeginPlay
  (Variables|Default|SetMove_right (Math|Random|RandomBool))
  (CallFunction|FacingDirection))

(event EventTick
  (params (DeltaSeconds :type Float%20%28single-precision%29))
  (CallFunction|UpdateAnimation)
  (Pawn|Input|AddMovementInput "1.000000,0.000000,0.000000" (select (Variables|Default|GetMove_right) 0.2 -0.2) false))

(fn ConstructionScript
  (|CallParentFunction))

(fn EnemyDead
  (bind _charactermovement (Variables|Character|GetCharacterMovement))
  (|CallParentFunction)
  (Variables|/Script/Engine.MovementComponent|SetVelocity _charactermovement "0, 0, 0")
  (Components|Movement|StopMovementImmediately _charactermovement)
  (Class|PrimitiveComponent|SetAllPhysicsLinearVelocity (Variables|Default|GetCapsuleComponent) "0, 0, 0" false)
  (Input|DisableInput (Game|GetPlayerController 0))
  (Physics|SetSimulatePhysics (Variables|Default|GetCapsuleComponent) true)
  (Physics|AddImpulse (Variables|Default|GetCapsuleComponent) (Math|Vector|MakeVector 0.0 0.0 4e+02) "None" true)
  (Collision|SetCollisionResponsetoAllChannels (Variables|Default|GetCapsuleComponent) "ECR_Ignore")
  (bind _asbp_mario (Utilities|Casting|CastToBP_Mario (Game|GetPlayerCharacter 0)))
  (Default|UpdadeKill _asbp_mario 1))

(fn FacingDirection
  (bind _sprite (Variables|Default|GetSprite))
  (bind _returnvalue (Transformation|GetWorldScale _sprite))
  (Transformation|SetWorldScale3D (Variables|Default|GetSprite) (Math|Vector|MakeVector (* (Math|Float|Absolute(Float) (.x _returnvalue)) (select (Variables|Default|GetMove_right) 1.0 -1.0)) (.y _returnvalue) (.z _returnvalue))))