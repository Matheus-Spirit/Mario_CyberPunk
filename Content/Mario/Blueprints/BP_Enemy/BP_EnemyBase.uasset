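; BP_EnemyBase is a base enemy for a Mario game, providing health, damage and sprite animation.
; Construction sets health to the default, and AnyDamage subtracts clamped damage, flags death at zero and calls EnemyDead, which is empty here.
; UpdateAnimation switches the flipbook between Walk and Idle by velocity while grounded, though nothing in this file calls it.
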(event Game|Damage|EventAnyDamage
  (params (Damage :type Float%20%28single-precision%29) (DamageType :type Damage%20Type%20Object%20Reference) (InstigatedBy :type Controller%20Object%20Reference) (DamageCauser :type Actor%20Object%20Reference))
  ;[1 1 1] Sistema de vida e de dano
  (Variables|Default|SetHeath (Math|Float|Clamp(Float) (- (Variables|Default|GetHeath) Damage) 0.0 (Variables|Default|GetDefaut%20Health)))
  (if (<= (Variables|Default|GetHeath) 0.0)
    (Variables|Default|SetIsDeath? true)
    (CallFunction|EnemyDead)))

(fn ConstructionScript
  (Variables|Default|SetHeath (Variables|Default|GetDefaut%20Health)))

(fn UpdateAnimation
  (if (AI|Components|NavMovement|IsMovingonGround (Variables|Character|GetCharacterMovement))
    (if (> (Math|Vector|VectorLength (Transformation|GetVelocity)) 0.0)
      (Sprite|SetFlipbook (Variables|Default|GetSprite) "/Game/Paper_2D/FlipBook/Gumba/Walk.Walk")
      (else
        (Sprite|SetFlipbook (Variables|Default|GetSprite) "/Game/Paper_2D/FlipBook/Gumba/Idle.Idle")))))

(fn EnemyDead)